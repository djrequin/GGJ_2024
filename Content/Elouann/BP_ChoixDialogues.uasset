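; BP_ChoixDialogues is a dialogue-choice manager that creates the category widget and relays its effects to the world.
; On BeginPlay it passes itself, three next-dialogue themes and three endings to WB_Category, then registers as the player character's Referent.
; Events move the mother (Daronne) by a modifier and spawn a gift at a target transform.
; MoveLeft and MoveRight respectively show and collapse both dialogue widgets when flagged visible.
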(event `self.ReceiveBeginPlay`
  (bind _returnvalue (`|CreateWidget` "/Game/Elouann/WB_Category.WB_Category_C"))
  (set `/Game/Elouann/WB_Category.HighRef` self _returnvalue)
  (set `/Game/Elouann/WB_Category.Theme1_NextDialogue` (`self.Prochain tex1`) _returnvalue)
  (set `/Game/Elouann/WB_Category.Theme2_NextDialogue` (`self.Prochain tex2`) _returnvalue)
  (set `/Game/Elouann/WB_Category.Theme3_NextDialogue` (`self.Prochain tex3`) _returnvalue)
  (set `self.createdWidget` _returnvalue)
  (set `/Game/Elouann/WB_Category.FinBonne` (`self.FinBonne`) _returnvalue)
  (set `/Game/Elouann/WB_Category.FinMoyenne` (`self.FinMoyenne`) _returnvalue)
  (set `/Game/Elouann/WB_Category.FinNul` (`self.FinNul`) _returnvalue)
  (`UserWidget.AddToViewport` _returnvalue 0)
  (`KismetSystemLibrary.Delay` 0.2)
  (bind _asbp_third_person_character (cast `/Game/ThirdPerson/Blueprints/BP_ThirdPersonCharacter` (`GameplayStatics.GetPlayerCharacter` 0)))
  (set `/Game/ThirdPerson/Blueprints/BP_ThirdPersonCharacter.Referent` self _asbp_third_person_character))

(event `MotherAngry`
  (params (Modifier :type "Float (double-precision)"))
  (`/Game/Elouann/BP_Daronne.Move` (`self.Daronne`) Modifier))

(event `SpawnGift`
  (`|SpawnActorFromClass` (`self.Cadeau`) (`SceneComponent.K2_GetComponentToWorld` (`self.Target`)) "Undefined" "MultiplyWithRoot" null null))

(event `MoveLeft`
  (bind _createdwidget (`self.createdWidget`))
  (bind _tempcreated_widget (`self.TempCreated Widget`))
  (set `self.TempCreated Widget` _createdwidget)
  (bind _output_get (set `self.TempCreated Widget 2` (`/Game/Elouann/WB_Category.CreatedWidget2` _createdwidget)))
  (`/Engine/EditorBlueprintResources/StandardMacros.IsValid` _tempcreated_widget
    (:`Is Valid`
      (if (`/Game/Elouann/WB_Category.visible` _tempcreated_widget)
        (`Widget.SetVisibility` _tempcreated_widget "Visible")))
    (:`Is Not Valid`
      _))
  (`/Engine/EditorBlueprintResources/StandardMacros.IsValid` _output_get
    (:`Is Valid`
      (if (`/Game/Elouann/WB_Dialogue.visible` _output_get)
        (`Widget.SetVisibility` _output_get "Visible")
        (`Widget.SetVisibility` _output_get "SelfHitTestInvisible")))))

(event `MoveRight`
  (bind _createdwidget (`self.createdWidget`))
  (bind _tempcreated_widget (`self.TempCreated Widget`))
  (set `self.TempCreated Widget` _createdwidget)
  (bind _output_get (set `self.TempCreated Widget 2` (`/Game/Elouann/WB_Category.CreatedWidget2` _createdwidget)))
  (`/Engine/EditorBlueprintResources/StandardMacros.IsValid` _tempcreated_widget
    (:`Is Valid`
      (if (`/Game/Elouann/WB_Category.visible` _tempcreated_widget)
        (`Widget.SetVisibility` _tempcreated_widget "Collapsed")))
    (:`Is Not Valid`
      _))
  (`/Engine/EditorBlueprintResources/StandardMacros.IsValid` _output_get
    (:`Is Valid`
      (if (`/Game/Elouann/WB_Dialogue.visible` _output_get)
        (`Widget.SetVisibility` _output_get "Collapsed")))))

(fn `UserConstructionScript`)