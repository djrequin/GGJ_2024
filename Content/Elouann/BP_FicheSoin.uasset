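; BP_FicheSoin is an actor that reveals a text description when the cursor hovers over its cube.
; On BeginPlay it copies its Description variable into a TextRender, hides it and turns on mouse-over events for the first player controller.
; The cube's begin and end cursor-over events then show and hide the TextRender, along with any child components.
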(event `self.ReceiveBeginPlay`
  (`TextRenderComponent.K2_SetText` (`self.TextRender`) (`self.Description`))
  (`SceneComponent.SetHiddenInGame` (`self.TextRender`) true true)
  (set `PlayerController.bEnableMouseOverEvents` true (`GameplayStatics.GetPlayerController` 0)))

(event `self.Cube.OnBeginCursorOver`
  (params (TouchedComponent :type "PrimitiveComponent Object Reference"))
  (`SceneComponent.SetHiddenInGame` (`self.TextRender`) false true))

(event `self.Cube.OnEndCursorOver`
  (params (TouchedComponent :type "PrimitiveComponent Object Reference"))
  (`SceneComponent.SetHiddenInGame` (`self.TextRender`) true true))

(fn `UserConstructionScript`)