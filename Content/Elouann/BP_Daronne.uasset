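; BP_Daronne is a character Blueprint whose skeletal mesh slides between its starting position and a Target point as other logic calls its Move event.
; Move accumulates input into a clamped Place value, normalized into a single blend alpha.
; That alpha interpolates the mesh position, drives an Alpha material parameter on both eye components (Oeil1, Oeil2) and shifts the eyes along their local Y axis.
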(event `self.ReceiveBeginPlay`
  (set `self.BaseLocationRelative` (`SceneComponent.RelativeLocation` (`self.SkeletalMesh`)))
  (set `self.TargetLocation` (`SceneComponent.RelativeLocation` (`self.Target`))))

(event `Move`
  (params (Movement :type "Float (double-precision)"))
  (bind _oeil2 (`self.Oeil2`))
  (bind _oeil1 (`self.Oeil1`))
  (bind _output_get (set `self.Place` (`KismetMathLibrary.FClamp` (+ Movement (`self.Place`)) -20.0 0.0)))
  (bind _returnvalue (/ (`KismetMathLibrary.Abs` _output_get) 20.0))
  (`SceneComponent.K2_SetRelativeLocation` (`self.SkeletalMesh`) (`KismetMathLibrary.VLerp` (`self.BaseLocationRelative`) (`self.TargetLocation`) _returnvalue) false false)
  (`MeshComponent.SetScalarParameterValueOnMaterials` _oeil1 "Alpha" _returnvalue)
  (`MeshComponent.SetScalarParameterValueOnMaterials` _oeil2 "Alpha" _returnvalue)
  (bind _returnvalue_2 (`KismetMathLibrary.Lerp` 7.0 11.0 _returnvalue))
  (`SceneComponent.K2_SetRelativeLocation` _oeil1 (`KismetMathLibrary.MakeVector` 5.5 _returnvalue_2 125.0) false false)
  (`SceneComponent.K2_SetRelativeLocation` _oeil2 (`KismetMathLibrary.MakeVector` -5.5 _returnvalue_2 125.0) false false))

(fn `UserConstructionScript`)